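; Game mode for a ship shooter that tallies player and enemy deaths and shows Win or TryAgain when either reaches TargetDeath.
; Deaths update the InGameUI and trigger respawns, with each new enemy at a random Y and stronger through an iteration counter.
; A countdown restarts on spawns, banking leftover seconds into Score.
; PlayerLose and EnemyLose are named inversely: PlayerLose shows Win, EnemyLose shows TryAgain.
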(event Custom|RespawnEnemy
  (params (CustomTime :type Float%20%28single-precision%29))
  (Audio|PlaySound2D "/Game/Audio/Hit.Hit" 1.0 1.0 0.0 0 0)
  (Variables|Default|SetEnemyDeath (+ (Variables|Default|GetEnemyDeath) 1))
  (CallFunction|UpdateScore)
  (if (Variables|Default|GetEnemyRespawn)
    (Utilities|Time|SetTimerbyFunctionName 0 "SpawnEnemy" CustomTime)))

(event Custom|Lose
  (Variables|Default|SetPlayerDeath (+ (Variables|Default|GetPlayerDeath) 1))
  (CallFunction|UpdateScore)
  (bind _outactors (Actor|GetAllActorsOfClass "/Game/Blueprints/PlayerShip.PlayerShip_C"))
  (Utilities|IsValid (Utilities|Array|Get(acopy) _outactors)
    (:Is%20Valid
      (Audio|PlaySound2D "/Game/Audio/Hit.Hit" 1.0 1.0 0.0 0 0)
      (if (Variables|Default|GetPlayerRespawn)
        (Default|DestroyShip (Utilities|Array|Get(acopy) _outactors))
        (Game|SpawnActorfromClass "/Game/Blueprints/PlayerShip.PlayerShip_C" (Math|Transform|MakeTransform "0, 0,80.000000") "AlwaysSpawn" 0 0)
        (CallFunction|ResetTimer 2e+01)
        (CallFunction|UpdateScore)))))

(event Custom|ResetTimer
  (params (Time :type Float%20%28single-precision%29))
  (Variables|Default|SetScore (+ (Math|Float|Truncate (Utilities|Time|GetTimerRemainingTimebyHandle (Variables|Default|GetTimer))) (Variables|Default|GetScore)))
  (bind _returnvalue (Utilities|Time|SetTimerbyEvent (EventDispatchers|CreateEvent :!event Custom|DeathByTimer) Time))
  (Variables|Default|SetTimer _returnvalue))

(event Custom|UpdateScore
  (bind _ingameoptions (Variables|Default|GetInGameOptions))
  (Utilities|IsValid _ingameoptions
    (:Is%20Valid
      (Variables|/Game/InGameUI.InGameUI_C|SetHScore _ingameoptions (Variables|Default|GetPlayerDeath))
      (Variables|/Game/InGameUI.InGameUI_C|SetSScore _ingameoptions (Variables|Default|GetEnemyDeath))
      (CallFunction|SubmitWinbyScore))))

(event Custom|SubmitWinByScore
  (if (>= (Variables|Default|GetEnemyDeath) (Variables|Default|GetTargetDeath))
    (CallFunction|PlayerLose)
    (elif (>= (Variables|Default|GetPlayerDeath) (Variables|Default|GetTargetDeath))
      (CallFunction|EnemyLose))))

(event Custom|PlayerLose
  (Utilities|FlowControl|DoOnce false
    (:Completed
      (Variables|Default|SetPlayerRespawn false)
      (bind _returnvalue (UserInterface|CreateWidget "/Game/Win.Win_C"))
      (UserInterface|Viewport|AddtoViewport _returnvalue 0))))

(event Custom|EnemyLose
  (Utilities|FlowControl|DoOnce false
    (:Completed
      (Variables|Default|SetEnemyRespawn false)
      (bind _returnvalue (UserInterface|CreateWidget "/Game/TryAgain.TryAgain_C"))
      (UserInterface|Viewport|AddtoViewport _returnvalue 0))))

(event Custom|DeathByTimer
  (Variables|Default|SetPlayerDeath (+ (Variables|Default|GetPlayerDeath) 1))
  (CallFunction|UpdateScore)
  (bind _outactors (Actor|GetAllActorsOfClass "/Game/Blueprints/PlayerShip.PlayerShip_C"))
  (if (Utilities|IsValid (Utilities|Array|Get(acopy) _outactors))
    (Default|DestroyShip (Utilities|Array|Get(acopy) _outactors))
    (Game|SpawnActorfromClass "/Game/Blueprints/PlayerShip.PlayerShip_C" (Math|Transform|MakeTransform "0, 0,80.000000") "AlwaysSpawn" 0 0)
    (CallFunction|ResetTimer 22.0)))

(event EventBeginPlay
  (CallFunction|SpawnEnemy)
  (bind _returnvalue (UserInterface|CreateWidget "/Game/InGameUI.InGameUI_C" (Game|GetPlayerController 0)))
  (UserInterface|Viewport|AddtoViewport _returnvalue 0)
  (Variables|/Game/InGameUI.InGameUI_C|SetGM _returnvalue self)
  (Audio|PlaySound2D "/Game/Audio/Derp_Nugget__mp3cut_net_.Derp_Nugget__mp3cut_net_" 1.0 1.0 0.0 0 0)
  (Variables|Default|SetInGameOptions _returnvalue)
  (CallFunction|UpdateScore))

(event EventTick
  (params (DeltaSeconds :type Float%20%28single-precision%29)))

(fn ConstructionScript)

(fn SpawnEnemy
  (bind _timer (Variables|Default|GetTimer))
  (bind _output_get (Variables|Default|SetEnemyIteration (+ (Variables|Default|GetEnemyIteration) 1)))
  (Game|SpawnActorfromClass "/Game/Blueprints/BP_EnemyP.BP_EnemyP_C" (Math|Transform|MakeTransform (Math|Vector|MakeVector 1.9e+03 (Math|Random|RandomFloatinRange -645.0 645.0) 2e+01) "0,180.000000, 0") "Undefined" 0 (/ _output_get 3) (/ _output_get 3) (/ _output_get 3) 0)
  (if (Utilities|Time|IsValidTimerHandle _timer)
    (CallFunction|ResetTimer (+ (/ (Utilities|Time|GetTimerRemainingTimebyHandle _timer) 1e+01) 2e+01))
    (else
      (CallFunction|ResetTimer 2e+01))))