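; Projectile actor that knocks physics objects it hits and then destroys itself.
; Its construction script sets both the initial and max speed of ProjectileMovement from the NewSpeed variable.
; On Hit, it applies an impulse scaled from its velocity at its location to any other simulating component, and is destroyed whatever it struck.
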(event EventBeginPlay)

(event Collision|EventActorBeginOverlap
  (params (OtherActor :type Actor%20Object%20Reference)))

(event EventTick
  (params (DeltaSeconds :type Float%20%28single-precision%29)))

(event Collision|EventHit
  (params (MyComp :type Primitive%20Component%20Object%20Reference) (Other :type Actor%20Object%20Reference) (OtherComp :type Primitive%20Component%20Object%20Reference) (bSelfMoved :type Boolean) (HitLocation :type Vector :default "0, 0, 0") (HitNormal :type Vector :default "0, 0, 0") (NormalImpulse :type Vector :default "0, 0, 0") (Hit :type Hit%20Result%20Structure%20%28by%20ref%29))
  (Utilities|IsValid Other
    (:Is%20Valid
      (Utilities|IsValid OtherComp
        (:Is%20Valid
          (if (and (!= self Other) (Class|SceneComponent|IsAnySimulatingPhysics OtherComp))
            (Physics|AddImpulseatLocation OtherComp (* (Transformation|GetVelocity) 4e+01) (Transformation|GetActorLocation) "None")))
        (:Is%20Not%20Valid
          _)))
    (:Is%20Not%20Valid
      _))
  (Actor|DestroyActor))

(fn ConstructionScript
  (bind _projectilemovement (Variables|Default|GetProjectileMovement))
  (bind _output_get (Variables|/Script/Engine.ProjectileMovementComponent|SetInitialSpeed _projectilemovement (Variables|Default|GetNewSpeed)))
  (Variables|/Script/Engine.ProjectileMovementComponent|SetMaxSpeed _projectilemovement _output_get))