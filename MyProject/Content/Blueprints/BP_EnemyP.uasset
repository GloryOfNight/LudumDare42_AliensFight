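; Enemy actor for a shooter that weaves side to side, fires on its own and awards score when destroyed.
; MoveComponentTo repeats with alternating direction and random duration, while randomly timed shots rarely use an alternate projectile; the twin-shot branch is disabled.
; Box hits lower Health and update the HP widget.
; At zero, a hit spawns debris and blood, pauses the BP_GameMode timer and requests a delayed respawn.
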(event OnComponentHit(Box)
  (params (HitComponent :type Primitive%20Component%20Object%20Reference) (OtherActor :type Actor%20Object%20Reference) (OtherComp :type Primitive%20Component%20Object%20Reference) (NormalImpulse :type Vector :default "0, 0, 0") (Hit :type Hit%20Result%20Structure%20%28by%20ref%29))
  (if (<= (Variables|Default|GetHealth) 0)
    (CallFunction|EnemyDestroy)
    (Actor|DestroyActor)
    (else
      (Variables|Default|SetHealth (- (Variables|Default|GetHealth) 1))
      (CallFunction|UpdateHealth))))

(event Custom|MoveComponent
  (bind _staticmesh (Variables|Default|GetStaticMesh))
  (bind _returnvalue (Transformation|GetRelativeTransform _staticmesh))
  (bind _location (Math|Transform|BreakTransform _returnvalue))
  (bind (_x _y _z) (Math|Vector|BreakVector _location))
  (if (Variables|Default|GetDirection)
    (Variables|Default|SetDirectionD 1.0)
    (else
      (Variables|Default|SetDirectionD -1.0)))
  (Components|MoveComponentTo (Variables|Default|GetStaticMesh) (Math|Vector|MakeVector _x (* 475.0 (Variables|Default|GetDirectionD)) _z) "0,180.000000, 0" false false (Variables|Default|GetTimeForOneDirectionMove) true)
  (Variables|Default|SetDirection (not (Variables|Default|GetDirection)))
  (Variables|Default|SetTimeForOneDirectionMove (Math|Random|RandomFloatinRange 0.9 1.5))
  (CallFunction|MoveComponent))

(event Custom|UpdateHealth
  (bind _ashp (Utilities|Casting|CastToHP (UserInterface|GetUserWidgetObject (Variables|Default|GetWidget))))
  (Variables|/Game/HP.HP_C|SetHP _ashp (+ (Variables|Default|GetHealth) 1))
  (Variables|/Game/HP.HP_C|SetMAXHP _ashp (+ (Variables|Default|GetMaxHealth) 1)))

(event EventBeginPlay
  (CallFunction|UpdateHealth)
  (CallFunction|MoveComponent)
  (Utilities|FlowControl|Delay 0.0)
  (Collision|SetCollisionEnabled (Variables|Default|GetBox) "QueryAndPhysics")
  (Rendering|SetVisibility (Variables|Default|GetStaticMesh) true false)
  (Utilities|FlowControl|Delay 0.7)
  (CallFunction|Fire))

(event Collision|EventActorBeginOverlap
  (params (OtherActor :type Actor%20Object%20Reference)))

(event EventTick
  (params (DeltaSeconds :type Float%20%28single-precision%29)))

(fn ConstructionScript
  (Collision|SetCollisionEnabled (Variables|Default|GetBox) "NoCollision"))

(fn EnemyDestroy
  (bind _returnvalue (Math|Random|RandomFloatinRange -5e+01 5e+01))
  (bind _returnvalue_2 (Math|Random|RandomFloatinRange -5e+01 5e+01))
  (bind _box (Variables|Default|GetBox))
  (bind _returnvalue_3 (Transformation|GetWorldLocation _box))
  (bind _returnvalue_4 (Math|Vector|MakeVector _returnvalue _returnvalue_2 0.0))
  (bind _returnvalue_5 (+ _returnvalue_3 _returnvalue_4 ""))
  (bind _returnvalue_6 (Math|Transform|MakeTransform _returnvalue_5))
  (for _index (range 0 6)
    (Game|SpawnActorfromClass "/Game/Blueprints/Trash.Trash_C" _returnvalue_6 "Undefined" 0 (Utilities|Select :Index _index :Option%200 "/Game/Sprite/Кусочек_1_Sprite.Кусочек_1_Sprite" :Option%201 "/Game/Sprite/Кусочек_2_Sprite.Кусочек_2_Sprite" :Option%202 "/Game/Sprite/Обломок_1_Sprite.Обломок_1_Sprite" :Option%203 "/Game/Sprite/Кусочек_1_Sprite.Кусочек_1_Sprite") 0))
  (Game|SpawnActorfromClass "/Game/Blueprints/Blood.Blood_C" _returnvalue_6 "Undefined" 0 0)
  (bind _asbp_game_mode (Utilities|Casting|CastToBP_GameMode (Game|GetGameMode)))
  (Utilities|Time|PauseTimerbyHandle (Variables|/Game/Blueprints/BP_GameMode.BP_GameMode_C|GetTimer _asbp_game_mode))
  (Variables|/Game/Blueprints/BP_GameMode.BP_GameMode_C|SetScore _asbp_game_mode (+ (Variables|/Game/Blueprints/BP_GameMode.BP_GameMode_C|GetScore _asbp_game_mode) 10))
  (Default|RespawnEnemy _asbp_game_mode (Math|Random|RandomFloatinRange 0.5 2.0))
  (bind _outactors (Actor|GetAllActorsOfClass "/Game/Blueprints/PlayerShip.PlayerShip_C")))

(fn Fire
  (bind _staticmesh (Variables|Default|GetStaticMesh))
  (bind _staticmesh_2 (Variables|Default|GetStaticMesh))
  (bind _projectilespeed (Variables|Default|GetProjectileSpeed))
  (bind _returnvalue (Transformation|GetWorldTransform _staticmesh_2))
  (bind _returnvalue_2 (Transformation|GetWorldLocation _staticmesh))
  (bind _location (Math|Transform|BreakTransform _returnvalue))
  (bind _returnvalue_3 (+ _location "-100.000000,0.000000,100.000000"))
  (bind _returnvalue_4 (Math|Transform|MakeTransform _returnvalue_3 "0.000000,180.000000, 0"))
  (if (Variables|Default|GetNotBlockFire)
    (Variables|Default|SetNotBlockFire false)
    (if false
      (Game|SpawnActorfromClass "/Game/Blueprints/Projectile.Projectile_C" (Math|Transform|MakeTransform (+ _returnvalue_2 "-220.000000,120.000000, 0") "0.000000,15.000000,0.000000") "AlwaysSpawn" 0 false _projectilespeed 0)
      (Game|SpawnActorfromClass "/Game/Blueprints/Projectile.Projectile_C" (Math|Transform|MakeTransform (+ _returnvalue_2 "-220.000000,-120.000000, 0") "0,7.500000,0.000000") "AlwaysSpawn" 0 false _projectilespeed 0)
      (Utilities|Time|SetTimerbyEvent (EventDispatchers|CreateEvent :!event Unblock) (Math|Random|RandomFloatinRange 1.0 3.0))
      (else
        (if (< (Math|Random|RandomFloatinRange 0.0 1e+02) 0.1)
          (Game|SpawnActorfromClass "/Game/Blueprints/ProjectileEnemy_2.ProjectileEnemy_2_C" _returnvalue_4 "AlwaysSpawn" 0 true _projectilespeed 0)
          (else
            (Game|SpawnActorfromClass "/Game/Blueprints/ProjectileEnemy.ProjectileEnemy_C" _returnvalue_4 "AlwaysSpawn" 0 true 1e+03 0)))
        (Utilities|Time|SetTimerbyEvent (EventDispatchers|CreateEvent :!event Unblock) (Math|Random|RandomFloatinRange 0.2 0.7))))))

(fn Unblock
  (Variables|Default|SetNotBlockFire true)
  (CallFunction|Fire))