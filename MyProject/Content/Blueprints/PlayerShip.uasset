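; Player-controlled Paper2D ship that slides sideways within fixed bounds, shoots and takes damage.
; Fire always spawns a five-projectile fan (single-shot branch is unreachable, SpecialAttack unused), then a timer calls UnlockCannon, which refires while fire is held.
; Cylinder hits decrement Health and update the HP widget, or call Lose on BP_GameMode once Health is zero.
; DestroyShip scatters debris and blood before destroying the actor, but nothing here calls it.
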(event OnComponentHit(StaticMesh)
  (params (HitComponent :type Primitive%20Component%20Object%20Reference) (OtherActor :type Actor%20Object%20Reference) (OtherComp :type Primitive%20Component%20Object%20Reference) (NormalImpulse :type Vector :default "0, 0, 0") (Hit :type Hit%20Result%20Structure%20%28by%20ref%29)))

(event OnComponentHit(Cylinder)
  (params (HitComponent :type Primitive%20Component%20Object%20Reference) (OtherActor :type Actor%20Object%20Reference) (OtherComp :type Primitive%20Component%20Object%20Reference) (NormalImpulse :type Vector :default "0, 0, 0") (Hit :type Hit%20Result%20Structure%20%28by%20ref%29))
  (if (<= (Variables|Default|GetHealth) 0)
    (Variables|Default|SetHealth 0)
    (bind _asbp_game_mode (Utilities|Casting|CastToBP_GameMode (Game|GetGameMode)))
    (Default|Lose _asbp_game_mode)
    (else
      (Variables|Default|SetHealth (- (Variables|Default|GetHealth) 1))
      (CallFunction|UpdateHealth))))

(event OnComponentBeginOverlap(Box)
  (params (OverlappedComponent :type Primitive%20Component%20Object%20Reference) (OtherActor :type Actor%20Object%20Reference) (OtherComp :type Primitive%20Component%20Object%20Reference) (OtherBodyIndex :type Integer) (bFromSweep :type Boolean) (SweepResult :type Hit%20Result%20Structure%20%28by%20ref%29))
  (Development|PrintString "Hello"))

(event Custom|UpdateHealth
  (bind _ashp (Utilities|Casting|CastToHP (UserInterface|GetUserWidgetObject (Variables|Default|GetWidget))))
  (Variables|/Game/HP.HP_C|SetHP _ashp (Variables|Default|GetHealth))
  (Variables|/Game/HP.HP_C|SetMAXHP _ashp (Variables|Default|GetMaxHealth)))

(event Custom|PlayReloadSound
  (Audio|PlaySound2D "/Game/Audio/Reload.Reload" 1.0 1.0 0.0 0 0))

(event EventBeginPlay
  (Variables|Default|SetHealth (Variables|Default|GetMaxHealth))
  (CallFunction|UpdateHealth))

(event Collision|EventActorBeginOverlap
  (params (OtherActor :type Actor%20Object%20Reference)))

(event EventTick
  (params (DeltaSeconds :type Float%20%28single-precision%29))
  (bind _papersprite (Variables|Default|GetPaperSprite))
  (bind _papersprite_2 (Variables|Default|GetPaperSprite))
  (bind _movementspeed (Variables|Default|GetMovementSpeed))
  (bind _returnvalue (Transformation|GetWorldLocation _papersprite_2))
  (bind _returnvalue_2 (* DeltaSeconds _movementspeed))
  (bind _y (Math|Vector|BreakVector _returnvalue))
  (if (Variables|Default|GetRightMove)
    (if (< _y 475.0)
      (Transformation|AddWorldOffset _papersprite (Math|Vector|MakeVector 0.0 _returnvalue_2 0.0) false true))
    (elif (Variables|Default|GetLeftMove)
      (if (not (< _y -475.0))
        (Transformation|AddWorldOffset _papersprite (Math|Vector|MakeVector 0.0 (* _returnvalue_2 -1.0) 0.0) false true)))))

(event Input|KeyboardEvents|Left
  (params (Key :type Key%20Structure))
  (:Pressed
    (Variables|Default|SetLeftMove true))
  (:Released
    (Variables|Default|SetLeftMove false)))

(event Input|KeyboardEvents|Right
  (params (Key :type Key%20Structure))
  (:Pressed
    (Variables|Default|SetRightMove true))
  (:Released
    (Variables|Default|SetRightMove false)))

(event Input|KeyboardEvents|Up
  (params (Key :type Key%20Structure))
  (:Pressed
    (Variables|Default|SetToggleFire true)
    (CallFunction|Fire))
  (:Released
    (Variables|Default|SetToggleFire false)))

(event Input|KeyboardEvents|SpaceBar
  (params (Key :type Key%20Structure))
  (:Pressed
    (Variables|Default|SetToggleFire true)
    (CallFunction|Fire))
  (:Released
    (Variables|Default|SetToggleFire false)))

(event Input|MouseEvents|LeftMouseButton
  (params (Key :type Key%20Structure))
  (:Pressed
    (Variables|Default|SetToggleFire true)
    (CallFunction|Fire))
  (:Released
    (Variables|Default|SetToggleFire false)))

(event Input|KeyboardEvents|Z
  (params (Key :type Key%20Structure))
  (:Pressed
    (Variables|Default|SetSpecialAttack true))
  (:Released
    (Variables|Default|SetSpecialAttack false)))

(fn ConstructionScript)

(fn Fire
  (bind _projectilespeed (Variables|Default|GetProjectileSpeed))
  (bind _papersprite (Variables|Default|GetPaperSprite))
  (bind _returnvalue (Transformation|GetWorldLocation _papersprite))
  (if (Variables|Default|GetNotBlockFire)
    (Variables|Default|SetNotBlockFire false)
    (Audio|PlaySound2D "/Game/Audio/Shoot.Shoot" 1.0 1.0 0.0 0 0)
    (if true
      (Game|SpawnActorfromClass "/Game/Blueprints/Projectile.Projectile_C" (Math|Transform|MakeTransform (+ _returnvalue "150.000000,-80.000000, 0") "0.000000,-7.500000,0.000000") "AlwaysSpawn" 0 false _projectilespeed 0)
      (Game|SpawnActorfromClass "/Game/Blueprints/Projectile.Projectile_C" (Math|Transform|MakeTransform (+ _returnvalue "150.000000,-37.000000, 0") "0,-2.500000,0.000000") "AlwaysSpawn" 0 false _projectilespeed 0)
      (Game|SpawnActorfromClass "/Game/Blueprints/Projectile.Projectile_C" (Math|Transform|MakeTransform (+ _returnvalue "150.000000,-3.000000, 0")) "AlwaysSpawn" 0 false _projectilespeed 0)
      (Game|SpawnActorfromClass "/Game/Blueprints/Projectile.Projectile_C" (Math|Transform|MakeTransform (+ _returnvalue "150.000000,43.000000, 0") "0,2.500000,0.000000") "AlwaysSpawn" 0 false _projectilespeed 0)
      (Game|SpawnActorfromClass "/Game/Blueprints/Projectile.Projectile_C" (Math|Transform|MakeTransform (+ _returnvalue "150.000000,80.000000, 0") "0,7.500000,0.000000") "AlwaysSpawn" 0 false _projectilespeed 0)
      (Utilities|Time|SetTimerbyFunctionName 0 "UnlockCannon" 2.0)
      (Utilities|Time|SetTimerbyEvent (EventDispatchers|CreateEvent :!event Custom|PlayReloadSound) 1.3)
      (else
        (Game|SpawnActorfromClass "/Game/Blueprints/Projectile.Projectile_C" (Math|Transform|MakeTransform (+ (Transformation|GetWorldLocation (Variables|Default|GetPaperSprite)) "100.000000,0.000000, 0")) "Undefined" 0 false 5e+03 0)
        (Utilities|Time|SetTimerbyFunctionName 0 "UnlockCannon" 0.3)))))

(fn UnlockCannon
  (Variables|Default|SetNotBlockFire true)
  (if (Variables|Default|GetToggleFire)
    (CallFunction|Fire)))

(fn DestroyShip
  (bind _papersprite (Variables|Default|GetPaperSprite))
  (bind _returnvalue (Transformation|GetWorldLocation _papersprite))
  (bind _returnvalue_2 (Math|Transform|MakeTransform _returnvalue))
  (bind (_location _rotation _scale) (Math|Transform|BreakTransform _returnvalue_2))
  (for _index (range 0 3)
    (Game|SpawnActorfromClass "/Game/Blueprints/Trash.Trash_C" (Math|Transform|MakeTransform (+ _location (Math|Vector|MakeVector (Math|Random|RandomFloatinRange -1.5e+02 1.5e+02) (Math|Random|RandomFloatinRange -1.5e+02 1.5e+02) 0.0)) _rotation _scale) "Undefined" 0 (Utilities|Select :Index _index :Option%200 "/Game/Sprite/Кусочек_1_Sprite.Кусочек_1_Sprite" :Option%201 "/Game/Sprite/Кусочек_2_Sprite.Кусочек_2_Sprite" :Option%202 "/Game/Sprite/Обломок_1_Sprite.Обломок_1_Sprite" :Option%203 "/Game/Sprite/Кусочек_1_Sprite.Кусочек_1_Sprite") 0))
  (Game|SpawnActorfromClass "/Game/Blueprints/Blood.Blood_C" _returnvalue_2 "Undefined" 0 0)
  (Actor|DestroyActor))