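; Game mode for a ship shooter that runs enemy waves, the countdown, score and loss flow.
; SpawnEnemy places a BP_EnemyP at random Y with stats scaled by spawn count, and RespawnEnemy delays the next spawn.
; Each spawn restarts the countdown with a leftover-time bonus, adding remaining seconds to Score.
; Lose decrements PlayerShip health and restarts the timer, or at zero health shows TryAgain and destroys the ship.
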(event Custom|RespawnEnemy
  (params (CustomTime :type Float%20%28single-precision%29))
  (Utilities|Time|SetTimerbyFunctionName 0 "SpawnEnemy" CustomTime))

(event Custom|Lose
  (bind _outactors (Actor|GetAllActorsOfClass "/Game/Blueprints/PlayerShip.PlayerShip_C"))
  (Utilities|IsValid (Utilities|Array|Get(acopy) _outactors)
    (:Is%20Valid
      (if (<= (Variables|/Game/Blueprints/PlayerShip.PlayerShip_C|GetHealth (Utilities|Array|Get(acopy) _outactors)) 0)
        (Utilities|FlowControl|DoOnce false
          (:Completed
            (bind _returnvalue (UserInterface|CreateWidget "/Game/TryAgain.TryAgain_C"))
            (UserInterface|Viewport|AddtoViewport _returnvalue 0)
            (bind _outactors_2 (Actor|GetAllActorsOfClass "/Game/Blueprints/PlayerShip.PlayerShip_C"))
            (Utilities|Time|PauseTimerbyHandle (Variables|Default|GetTimer))
            (Utilities|IsValid (Utilities|Array|Get(acopy) _outactors_2)
              (:Is%20Valid
                (Actor|DestroyActor (Utilities|Array|Get(acopy) _outactors_2))))))
        (else
          (Variables|/Game/Blueprints/PlayerShip.PlayerShip_C|SetHealth (Utilities|Array|Get(acopy) _outactors) (- (Variables|/Game/Blueprints/PlayerShip.PlayerShip_C|GetHealth (Utilities|Array|Get(acopy) _outactors)) 1))
          (CallFunction|ResetTimer 2e+01)
          (Default|UpdateHealth (Utilities|Array|Get(acopy) _outactors)))))))

(event Custom|ResetTimer
  (params (Time :type Float%20%28single-precision%29))
  (Variables|Default|SetScore (+ (Math|Float|Truncate (Utilities|Time|GetTimerRemainingTimebyHandle (Variables|Default|GetTimer))) (Variables|Default|GetScore)))
  (bind _returnvalue (Utilities|Time|SetTimerbyEvent (EventDispatchers|CreateEvent :!event Custom|Lose) Time))
  (Variables|Default|SetTimer _returnvalue))

(event EventBeginPlay
  (CallFunction|SpawnEnemy)
  (bind _returnvalue (UserInterface|CreateWidget "/Game/InGameUI.InGameUI_C" (Game|GetPlayerController 0)))
  (UserInterface|Viewport|AddtoViewport _returnvalue 0)
  (Variables|/Game/InGameUI.InGameUI_C|SetGM _returnvalue self)
  (Audio|PlaySound2D "/Game/Audio/Derp_Nugget__mp3cut_net_.Derp_Nugget__mp3cut_net_" 1.0 1.0 0.0 0 0))

(event EventTick
  (params (DeltaSeconds :type Float%20%28single-precision%29)))

(fn ConstructionScript)

(fn SpawnEnemy
  (bind _timer (Variables|Default|GetTimer))
  (bind _output_get (Variables|Default|SetEnemyIteration (+ (Variables|Default|GetEnemyIteration) 1)))
  (Game|SpawnActorfromClass "/Game/Blueprints/BP_EnemyP.BP_EnemyP_C" (Math|Transform|MakeTransform (Math|Vector|MakeVector 1.9e+03 (Math|Random|RandomFloatinRange -645.0 645.0) 2e+01) "0,180.000000, 0") "Undefined" 0 (/ _output_get 3) (/ _output_get 3) (/ _output_get 3) 0)
  (if (Utilities|Time|IsValidTimerHandle _timer)
    (CallFunction|ResetTimer (+ (/ (Utilities|Time|GetTimerRemainingTimebyHandle _timer) 1e+01) 2e+01))
    (else
      (CallFunction|ResetTimer 2e+01))))